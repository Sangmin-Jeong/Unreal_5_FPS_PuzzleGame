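; Game instance that manages frontend and gameplay background music, keeping it alive across level transitions.
; Each track has play and stop functions, and playing one fades out the other before fading itself in.
; Audio components are created lazily as persistent 2D sounds, then reused, with a fade-in only when not already playing.
; Stop functions fade out by default or cut immediately when forced.
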(fn PlayGameplayMusic
  (CallFunction|StopFrontendMusic false)
  (Utilities|IsValid (Variables|Default|GetGameplayMusic)
    (:Is%20Valid
      ;[1 1 1] Play music if it is not playing
      (if (not (Audio|Components|Audio|IsPlaying (Variables|Default|GetGameplayMusic)))
        (Audio|Components|Audio|FadeIn (Variables|Default|GetGameplayMusic) 1.0 1.0 0.0 "Linear" :!class /Script/Engine.AudioComponent)))
    (:Is%20Not%20Valid
      ;[1 1 1] Create and play music
      (bind _returnvalue (Audio|CreateSound2D "/Game/Audio/Music/S_GameplayMusic.S_GameplayMusic" 1.0 1.0 0.0 0 true))
      (bind _output_get (Variables|Default|SetGameplayMusic _returnvalue))
      (Audio|Components|Audio|FadeIn _output_get 1.0 1.0 0.0 "Linear" :!class /Script/Engine.AudioComponent))))

(fn StopGameplayMusic
  (params (Force :type Boolean))
  ;[1 1 1] Stop music if it is playing
  (Utilities|IsValid (Variables|Default|GetGameplayMusic)
    (:Is%20Valid
      (if (Audio|Components|Audio|IsPlaying (Variables|Default|GetGameplayMusic))
        (if Force
          (Audio|Components|Audio|Stop (Variables|Default|GetGameplayMusic))
          (else
            (Audio|Components|Audio|FadeOut (Variables|Default|GetGameplayMusic) 1.0 0.0 "Linear" :!class /Script/Engine.AudioComponent)))))))

(fn PlayFrontendMusic
  (CallFunction|StopGameplayMusic false)
  (Utilities|IsValid (Variables|Default|GetFrontendMusic)
    (:Is%20Valid
      ;[1 1 1] Play music if it is not playing
      (if (not (Audio|Components|Audio|IsPlaying (Variables|Default|GetFrontendMusic)))
        (Audio|Components|Audio|FadeIn (Variables|Default|GetFrontendMusic) 1.0 1.0 0.0 "Linear" :!class /Script/Engine.AudioComponent)))
    (:Is%20Not%20Valid
      ;[1 1 1] Create and play music
      (bind _returnvalue (Audio|CreateSound2D "/Game/Audio/Music/S_FrontendMusic.S_FrontendMusic" 1.0 1.0 0.0 0 true))
      (bind _output_get (Variables|Default|SetFrontendMusic _returnvalue))
      (Audio|Components|Audio|FadeIn _output_get 1.0 1.0 0.0 "Linear" :!class /Script/Engine.AudioComponent))))

(fn StopFrontendMusic
  (params (Force :type Boolean))
  ;[1 1 1] Stop music if it is playing
  (Utilities|IsValid (Variables|Default|GetFrontendMusic)
    (:Is%20Valid
      (if (Audio|Components|Audio|IsPlaying (Variables|Default|GetFrontendMusic))
        (if Force
          (Audio|Components|Audio|Stop (Variables|Default|GetFrontendMusic))
          (else
            (Audio|Components|Audio|FadeOut (Variables|Default|GetFrontendMusic) 1.0 0.0 "Linear" :!class /Script/Engine.AudioComponent)))))))