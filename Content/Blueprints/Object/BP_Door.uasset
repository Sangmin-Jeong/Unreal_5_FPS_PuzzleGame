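; BP_Door is a switchable puzzle door that slides up when switched on and back down when switched off.
; DoorTimeline lerps the door mesh's relative Z, playing forward on SwitchOn and reversing on SwitchOff.
; SwitchOn uses an IsSwitching guard, cleared on timeline update, and updates game stats.
; A final door also fires the PuzzleMageGameMode final-door delegate on its first activation.
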(event Custom|SwitchOn
  ;[1 1 1] Door goes up when on, goes down when off
  (if (not (Variables|Default|GetIsSwitching))
    (Variables|Default|SetIsSwitching true)
    (Class|Door|UpdateGameStats)
    (if (Variables|Default|GetbIsFinalDoor)
      (if (Variables|Default|GetIsActiveCamActivated)
        (bind _newtrack_0 (Timeline|Door%20Timeline Play)
          (:Update
            (Transformation|SetRelativeLocation (Variables|Default|GetDoor) (Math|Vector|MakeVector 0.0 0.0 (Math|Float|Lerp 0.0 3e+02 _newtrack_0)) false false)
            (Variables|Default|SetIsSwitching false)))
        (else
          (bind _aspuzzle_mage_game_mode (Utilities|Casting|CastToPuzzleMageGameMode (Game|GetGameMode)))
          (Class|PuzzleMageGameMode|ExecuteFinalDoorDelegate _aspuzzle_mage_game_mode)
          (Variables|Default|SetIsActiveCamActivated true)
          (Timeline|Door%20Timeline Play)))
      (else
        (Timeline|Door%20Timeline Play)))))

(event Custom|SwitchOff
  ;[1 1 1] Door goes up when on, goes down when off
  (bind _newtrack_0 (Timeline|Door%20Timeline Reverse)
    (:Update
      (Transformation|SetRelativeLocation (Variables|Default|GetDoor) (Math|Vector|MakeVector 0.0 0.0 (Math|Float|Lerp 0.0 3e+02 _newtrack_0)) false false)
      (Variables|Default|SetIsSwitching false))))

(event EventBeginPlay
  (Components|StaticMesh|SetStaticMesh (Variables|Default|GetIcon) (Variables|Default|GetIconStaticMesh)))

(fn ConstructionScript)