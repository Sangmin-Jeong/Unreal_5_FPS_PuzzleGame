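; BP_MovableBlock is a block that uses particle VFX to hint to the player that it can be moved.
; Box overlap begin hides the Cascade particles for any overlapping actor.
; Overlap end, only for the active player character, restores the default dungeon material and shows the particles again.
; This graph contains no movement logic and never applies a highlight material.
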(event OnComponentBeginOverlap(BoxComponent)
  (params (OverlappedComponent :type Primitive%20Component%20Object%20Reference) (OtherActor :type Actor%20Object%20Reference) (OtherComp :type Primitive%20Component%20Object%20Reference) (OtherBodyIndex :type Integer) (bFromSweep :type Boolean) (SweepResult :type Hit%20Result%20Structure%20%28by%20ref%29))
  ;[1 1 1] Play VFX to give hint to player that it is a movable block
  (Development|SetHiddeninGame (Variables|Default|GetCascadeParticleSystem) true false))

(event OnComponentEndOverlap(BoxComponent)
  (params (OverlappedComponent :type Primitive%20Component%20Object%20Reference) (OtherActor :type Actor%20Object%20Reference) (OtherComp :type Primitive%20Component%20Object%20Reference) (OtherBodyIndex :type Integer))
  ;[1 1 1] Set to default color
  (if (== OtherActor (Class|MyBlueprintFunctionLibrary|GetActivePlayerCharacter))
    (Rendering|Material|SetMaterial (Variables|Default|GetStaticMeshComponent) 0 "/Game/PolygonDungeons/Materials/M_Dungeon_01.M_Dungeon_01")
    (Development|SetHiddeninGame (Variables|Default|GetCascadeParticleSystem) false false)))

(fn ConstructionScript)