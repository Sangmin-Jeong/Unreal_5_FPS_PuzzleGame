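; BP_MirrorWall is a wall that changes appearance when the active player character overlaps its box trigger.
; On begin overlap by the player, the mesh's first material slot switches to Transparency_Mat, and end overlap restores M_Dungeon_01.
; Any other overlapping actor gets the inverse swap, so it sets the dungeon material on entry and transparency on exit.
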(event OnComponentBeginOverlap(BoxComponent)
  (params (OverlappedComponent :type Primitive%20Component%20Object%20Reference) (OtherActor :type Actor%20Object%20Reference) (OtherComp :type Primitive%20Component%20Object%20Reference) (OtherBodyIndex :type Integer) (bFromSweep :type Boolean) (SweepResult :type Hit%20Result%20Structure%20%28by%20ref%29))
  (if (== OtherActor (Class|MyBlueprintFunctionLibrary|GetActivePlayerCharacter))
    (Rendering|Material|SetMaterial (Variables|Default|GetStaticMeshComponent) 0 "/Game/PolygonDungeons/Materials/Misc/Transparency_Mat.Transparency_Mat")
    (else
      (Rendering|Material|SetMaterial (Variables|Default|GetStaticMeshComponent) 0 "/Game/PolygonDungeons/Materials/M_Dungeon_01.M_Dungeon_01"))))

(event OnComponentEndOverlap(BoxComponent)
  (params (OverlappedComponent :type Primitive%20Component%20Object%20Reference) (OtherActor :type Actor%20Object%20Reference) (OtherComp :type Primitive%20Component%20Object%20Reference) (OtherBodyIndex :type Integer))
  (if (== OtherActor (Class|MyBlueprintFunctionLibrary|GetActivePlayerCharacter))
    (Rendering|Material|SetMaterial (Variables|Default|GetStaticMeshComponent) 0 "/Game/PolygonDungeons/Materials/M_Dungeon_01.M_Dungeon_01")
    (else
      (Rendering|Material|SetMaterial (Variables|Default|GetStaticMeshComponent) 0 "/Game/PolygonDungeons/Materials/Misc/Transparency_Mat.Transparency_Mat"))))

(fn ConstructionScript)