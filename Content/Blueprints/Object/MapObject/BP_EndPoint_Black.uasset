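; Level exit object that plays a sound, flags game data for saving and loads the next level when PuzzleMageCharacter overlaps it.
; The game instance supplies the next level data asset; without one it loads the outro after LastLevelReference, otherwise the main menu.
; Chapter and level indices of the next level unlock progress achievements once.
; The final-chapter achievement checks the current level on a separate branch, outside the character cast.
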(event Collision|EventActorBeginOverlap
  (params (OtherActor :type Actor%20Object%20Reference))
  (Utilities|FlowControl|Sequence
    (:then_0
      (Utilities|Casting|CastToPuzzleMageCharacter OtherActor)
      (Audio|PlaySound2D (Variables|Default|GetInteractionSound) 1.0 1.0 0.0 0 0)
      (bind _returnvalue (Class|MyBlueprintFunctionLibrary|GetGameInstance))
      (Class|MyGameInstance|SetShouldSaveGameData _returnvalue true)
      (Utilities|IsValid (Class|MyGameInstance|GetNextLevelDataAsset _returnvalue)
        (:Is%20Valid
          (Class|MyBlueprintFunctionLibrary|LoadLevelbyReferenceAfterDelay (Class|MyGameInstance|GetNextLevelDataAsset _returnvalue) true 0.35)
          ;[1 1 1] First Level Achievement
          (Utilities|FlowControl|Sequence
            (:then_0
              (if (not (Variables|Default|GetFirstLevelAchievementUnlocked))
                (bind _asbp_my_game_instance (Utilities|Casting|CastToBP_MyGameInstance (Game|GetGameInstance)))
                (if (== (Variables|/Script/PuzzleMage.LevelDataAsset|GetChapterIndex (Class|MyGameInstance|GetNextLevelDataAsset _asbp_my_game_instance)) 0)
                  (if (== (Variables|/Script/PuzzleMage.LevelDataAsset|GetLevelIndex (Class|MyGameInstance|GetNextLevelDataAsset _asbp_my_game_instance)) 2)
                    (Class|MyBlueprintFunctionLibrary|UnlockAchievement "FirstLevel")
                    (Variables|Default|SetFirstLevelAchievementUnlocked true)))))
            (:then_1
              ;[1 1 1] First Chapter Achievement
              (if (not (Variables|Default|GetFirstChapterlAchievementUnlocked))
                (bind _asbp_my_game_instance_2 (Utilities|Casting|CastToBP_MyGameInstance (Game|GetGameInstance)))
                (if (== (Variables|/Script/PuzzleMage.LevelDataAsset|GetChapterIndex (Class|MyGameInstance|GetNextLevelDataAsset _asbp_my_game_instance_2)) 1)
                  (if (== (Variables|/Script/PuzzleMage.LevelDataAsset|GetLevelIndex (Class|MyGameInstance|GetNextLevelDataAsset _asbp_my_game_instance_2)) 1)
                    (Class|MyBlueprintFunctionLibrary|UnlockAchievement "FirstChapter")
                    (Variables|Default|SetFirstChapterlAchievementUnlocked true)))))
            (:then_2
              ;[1 1 1] Second Chapter Achievement
              (if (not (Variables|Default|GetSecondChapterlAchievementUnlocked))
                (bind _asbp_my_game_instance_3 (Utilities|Casting|CastToBP_MyGameInstance (Game|GetGameInstance)))
                (if (== (Variables|/Script/PuzzleMage.LevelDataAsset|GetChapterIndex (Class|MyGameInstance|GetNextLevelDataAsset _asbp_my_game_instance_3)) 2)
                  (if (== (Variables|/Script/PuzzleMage.LevelDataAsset|GetLevelIndex (Class|MyGameInstance|GetNextLevelDataAsset _asbp_my_game_instance_3)) 1)
                    (Class|MyBlueprintFunctionLibrary|UnlockAchievement "SecondChapter")
                    (Variables|Default|SetSecondChapterlAchievementUnlocked true)))))))
        (:Is%20Not%20Valid
          (bind _returnvalue_2 (Class|MyBlueprintFunctionLibrary|GetGameInstance))
          (if (== (Class|MyGameInstance|GetCurrentLevelDataAsset _returnvalue_2) (Variables|Default|GetLastLevelReference))
            (Class|MyBlueprintFunctionLibrary|LoadLevelbyNameAfterDelay "OutroScene" true 0.35)
            (else
              (Class|MyBlueprintFunctionLibrary|LoadLevelbyNameAfterDelay "MainMenuScreen" true 0.35))))))
    (:then_1
      ;[1 1 1] Third Chapter and Clear game Achievement
      (if (not (Variables|Default|GetThirdChapterlAchievementUnlocked))
        (bind _asbp_my_game_instance_4 (Utilities|Casting|CastToBP_MyGameInstance (Game|GetGameInstance)))
        (if (and (== (Variables|/Script/PuzzleMage.LevelDataAsset|GetChapterIndex (Class|MyGameInstance|GetCurrentLevelDataAsset _asbp_my_game_instance_4)) 2) (== (Variables|/Script/PuzzleMage.LevelDataAsset|GetLevelIndex (Class|MyGameInstance|GetCurrentLevelDataAsset _asbp_my_game_instance_4)) 4))
          (Class|MyBlueprintFunctionLibrary|UnlockAchievement "ThirdChapter")
          (Variables|Default|SetThirdChapterlAchievementUnlocked true))))))

(event EventTick
  (params (DeltaSeconds :type Float%20%28single-precision%29)))

(fn ConstructionScript)