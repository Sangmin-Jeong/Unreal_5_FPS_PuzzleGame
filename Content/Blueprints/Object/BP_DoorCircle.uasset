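; Switch-driven puzzle door that swings its Door component open to 80 degrees yaw and displays a configurable icon mesh.
; SwitchOn updates game stats and plays a timeline after OpenDelay, guarded by IsSwitching, which clears on timeline updates.
; A final door also fires the game mode's final-door delegate on first activation.
; SwitchOff reverses the timeline after CloseDelay.
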(event Custom|SwitchOn
  ;[1 1 1] Door goes up when on, goes down when off
  (if (not (Variables|Default|GetIsSwitching))
    (Variables|Default|SetIsSwitching true)
    (Class|Door|UpdateGameStats)
    (if (Variables|Default|GetbIsFinalDoor)
      (if (Variables|Default|GetIsActiveCamActivated)
        _
        (else
          (bind _aspuzzle_mage_game_mode (Utilities|Casting|CastToPuzzleMageGameMode (Game|GetGameMode)))
          (Class|PuzzleMageGameMode|ExecuteFinalDoorDelegate _aspuzzle_mage_game_mode)
          (Variables|Default|SetIsActiveCamActivated true))))
    (Utilities|FlowControl|Delay (Variables|Default|GetOpenDelay))
    (bind _newtrack_0 (Timeline|Door%20Timeline Play)
      (:Update
        (Transformation|SetRelativeRotation (Variables|Default|GetDoor) (Math|Rotator|MakeRotator 0.0 0.0 (Math|Float|Lerp 0.0 8e+01 _newtrack_0)) false false)
        (Variables|Default|SetIsSwitching false)))))

(event Custom|SwitchOff
  ;[1 1 1] Door goes up when on, goes down when off
  (Utilities|FlowControl|Delay (Variables|Default|GetCloseDelay))
  (bind _newtrack_0 (Timeline|Door%20Timeline Reverse)
    (:Update
      (Transformation|SetRelativeRotation (Variables|Default|GetDoor) (Math|Rotator|MakeRotator 0.0 0.0 (Math|Float|Lerp 0.0 8e+01 _newtrack_0)) false false)
      (Variables|Default|SetIsSwitching false))))

(event EventBeginPlay
  (Components|StaticMesh|SetStaticMesh (Variables|Default|GetIcon) (Variables|Default|GetIconStaticMesh)))

(fn ConstructionScript)